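; Strategy game mode Blueprint that shows the end-of-match screen when the game is over.
; OnGameOver switches on the winning team, adding a winner widget to the viewport for the player team or a loser widget for the AI team, then sets UI-only input.
; Nodes that would show the mouse cursor are present but unreachable, and BeginPlay, Tick and the construction script are empty.
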(event `self.OnGameOver`
  (params (Winner :type "ETeam Enum" :default "Player"))
  (switch `ETeam` Winner
    (:`Player`
      (bind _returnvalue (`|CreateWidget` "/Game/Blueprints/WBP_GameOverWinner.WBP_GameOverWinner_C" (`GameplayStatics.GetPlayerController` 0)))
      (`UserWidget.AddToViewport` _returnvalue 0))
    (:`AI`
      (bind _returnvalue_2 (`|CreateWidget` "/Game/Blueprints/WBP_GameOverLoser.WBP_GameOverLoser_C" (`GameplayStatics.GetPlayerController` 0)))
      (`UserWidget.AddToViewport` _returnvalue_2 0)))
  (`WidgetBlueprintLibrary.SetInputMode_UIOnlyEx` (`GameplayStatics.GetPlayerController` 0) null))

(fn `UserConstructionScript`)