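; BP_UnitBase is a base unit Blueprint that handles a unit's health bar and floating damage feedback.
; Setup themes the WBP_HealthBar widget by UnitTeam and prints the unit's name and team.
; Health changes forward current and max health to that bar.
; Damage events spawn a BP_FloatingDamage actor at the given location and pass the truncated amount to its WBP_DamageText widget.
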(event `self.OnSetupHealthBar`
  (params (Team :type "ETeam Enum" :default "Player"))
  (bind _unitteam (`self.UnitTeam`))
  (bind _aswbp_health_bar (cast `/Game/Blueprints/WBP_HealthBar` (`WidgetComponent.GetUserWidgetObject` (`self.HealthBar`))))
  (`KismetSystemLibrary.PrintString` (`KismetStringLibrary.Concat_StrStr` (`KismetSystemLibrary.GetDisplayName` self) (`|GetEnumeratorNameAsString` _unitteam)))
  (`/Game/Blueprints/WBP_HealthBar.SetTheme` _aswbp_health_bar _unitteam))

(event `self.OnShowFloatingDamage`
  (params (DamageAmount :type "Float (single-precision)") (SpawnLocation :type "Vector Structure"))
  (bind _returnvalue (`|SpawnActorFromClass` "/Game/Blueprints/BP_FloatingDamage.BP_FloatingDamage_C" (`KismetMathLibrary.Conv_VectorToTransform` SpawnLocation) "Undefined" "MultiplyWithRoot" null null))
  (bind _aswbp_damage_text (cast `/Game/Blueprints/WBP_DamageText` (`WidgetComponent.GetWidget` (`/Game/Blueprints/BP_FloatingDamage.Widget` _returnvalue))))
  (`/Game/Blueprints/WBP_DamageText.SetDamageNumber` _aswbp_damage_text (`KismetMathLibrary.FTrunc` DamageAmount)))

(event `self.OnHealthChanged`
  (params (NewCurrentHealth :type "Float (single-precision)") (NewMaxHealth :type "Float (single-precision)"))
  (bind _aswbp_health_bar (cast `/Game/Blueprints/WBP_HealthBar` (`WidgetComponent.GetUserWidgetObject` (`self.HealthBar`))))
  (`/Game/Blueprints/WBP_HealthBar.HealtUpdate` _aswbp_health_bar NewCurrentHealth NewMaxHealth))

(fn `UserConstructionScript`)